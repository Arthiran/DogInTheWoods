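; BP_Pickup is a pickup actor that shows a pickup text prompt on the player character's HUD widget while that character is in range.
; Begin overlap casts the other actor to BP_Character and shows its PickupTextPanel, unless AlreadyPickedUp is set.
; End overlap hides the panel regardless of that flag.
; The graph only reads AlreadyPickedUp and contains no logic for the pickup itself.
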(event `self.ReceiveActorBeginOverlap`
  (params (OtherActor :type "Actor Object Reference"))
  (if (not (`self.AlreadyPickedUp`))
    (bind _asbp_character (cast `/Game/Blueprints/BP_Character` OtherActor))
    (`Widget.SetVisibility` (`/Game/Blueprints/Widgets/WBP_UI.PickupTextPanel` (`/Game/Blueprints/BP_Character.Widget` _asbp_character)) "Visible")))

(event `self.ReceiveActorEndOverlap`
  (params (OtherActor :type "Actor Object Reference"))
  (bind _asbp_character (cast `/Game/Blueprints/BP_Character` OtherActor))
  (`Widget.SetVisibility` (`/Game/Blueprints/Widgets/WBP_UI.PickupTextPanel` (`/Game/Blueprints/BP_Character.Widget` _asbp_character)) "Hidden"))

(fn `UserConstructionScript`)